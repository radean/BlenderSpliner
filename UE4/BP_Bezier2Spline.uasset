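; Actor that rebuilds its spline on BeginPlay from Bezier-style points in a data table.
; Rebuild adds each row as a local point, converting handle positions into tangents via swapped in/out fields and a Hermite scale.
; Raised points get a world-Z up vector.
; NotationPoints and CleanupNotation add and remove numbered distance labels, but neither is wired to run.
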(event `self.ReceiveBeginPlay`
  (`self.Rebuild`))

(fn `CleanupNotation`
  (for _index (range (`KismetArrayLibrary.Array_Length` (`self.TextRenderComp_Arr`)))
    (`ActorComponent.K2_DestroyComponent` (`|GetArrayItem` (`self.TextRenderComp_Arr`) _index))))

(fn `NotationPoints`
  (bind _spline (`self.Spline`))
  (bind (_remainder _returnvalue) (`KismetMathLibrary.FMod` (`SplineComponent.GetSplineLength` _spline) 160000.0))
  (for _index (range (+ _returnvalue 1))
    (bind _returnvalue_2 (`AddComponent|NODE_AddTextRenderComponent-0` :`RelativeTransform` (`KismetMathLibrary.Conv_VectorToTransform` (`SplineComponent.GetLocationAtDistanceAlongSpline` _spline (`self.DistanceGap`) "World"))))
    (`TextRenderComponent.K2_SetText` _returnvalue_2 (`KismetTextLibrary.Conv_IntToText` _index))
    (`KismetArrayLibrary.Array_Add` (`self.TextRenderComp_Arr`) _returnvalue_2)
    (set `self.DistanceGap` (+ (`self.DistanceGap`) 160000.0))
    (`KismetSystemLibrary.PrintString` (`KismetStringLibrary.Conv_IntToString` _returnvalue))))

(fn `Rebuild`
  (locals (L_CurrentIndex :type Integer) (Hermite :type "Float (double-precision)" :default 3.0) (L_Position :type "Vector Structure") (L_InTangent :type "Vector Structure") (L_OutTangent :type "Vector Structure"))
  (bind _l_position (`local.L_Position`))
  (bind (_l_position_x _l_position_y _l_position_z) (`KismetMathLibrary.BreakVector` (`local.L_Position`)))
  (bind _hermite (`local.Hermite`))
  (`SplineComponent.ClearSplinePoints` (`self.Spline`) true)
  (bind _outrownames (`DataTableFunctionLibrary.GetDataTableRowNames` (`self.TableSplinePoints`)))
  (for (_array_element _array_index) _outrownames
    (set `local.L_CurrentIndex` _array_index)
    (bind _returnvalue (`|GetDataTableRow` (`self.TableSplinePoints`) _array_element)
      (:`then`
        (bind (_position _intangent _outtangent) (break `/Game/Bezier2Spline/Data/Structs/FBezierPoints` _returnvalue))
        (set `local.L_Position` _position)
        (set `local.L_InTangent` _outtangent)
        (set `local.L_OutTangent` _intangent)
        (`SplineComponent.AddSplinePoint` (`self.Spline`) _l_position "Local" true)
        (`SplineComponent.SetTangentsAtSplinePoint` (`self.Spline`) (`local.L_CurrentIndex`) (* (- _l_position (`local.L_InTangent`)) _hermite) (* (- _l_position (`local.L_OutTangent`)) (* _hermite -1.0)) "Local" true)
        ;[1 1 1] Fix up vector for points off the floor
        (if (> _l_position_z 10.0)
          (`SplineComponent.SetUpVectorAtSplinePoint` (`self.Spline`) (`local.L_CurrentIndex`) (`KismetMathLibrary.MakeVector` 0.0 0.0 1.0) "World" true))))))

(fn `UserConstructionScript`
  (locals (L_CurrentIndex :type Integer)))